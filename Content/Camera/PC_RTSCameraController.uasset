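; RTS player controller that handles mouse-driven unit and building selection, move orders and unit production.
; Left click selects the building under the cursor and drives the HUD's marquee selection through press, hold and release messages.
; Right click sends the HUD's selected units to the clicked location and spawns a cursor effect there.
; ProduceUnit passes requests through ServerAddUnitToQueue to the building's production queue.
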(event `/Game/UnitSelection/Unit/BP_RTS_Interface.ClearSelectedBuilding`
  (bind _selectedbuilding (`self.SelectedBuilding`))
  ;[0.8826 1 0.6586] Deselect Building
  (`/Engine/EditorBlueprintResources/StandardMacros.IsValid` _selectedbuilding
    (:`Is Valid`
      (message `/Game/UnitSelection/Unit/BP_RTS_Interface.DeselectThis` _selectedbuilding)
      (set `self.SelectedBuilding` null))))

(event `self.ReceiveBeginPlay`
  ;[0.3262 1 0.9834] Show Mouse Cursor
  (`WidgetBlueprintLibrary.SetInputMode_GameAndUIEx` self null "DoNotLock" false)
  (set `self.bShowMouseCursor` true))

(event `self.ReceiveTick`
  (params (DeltaSeconds :type "Float (single-precision)"))
  ;[1 0.05734 0.4005] Select Unit
  (if (`self.isLeftMousePressed?`)
    (message `/Game/UnitSelection/Unit/BP_RTS_Interface.MarqueeHeld` (`self.GetHUD`))))

(event `Key|LeftMouseButton`
  (params (Key :type "Key Structure"))
  (bind _returnvalue (`self.GetHUD`))
  ;[1 0.05734 0.4005] Select Unit
  (:`Pressed`
    (set `self.isLeftMousePressed?` true)
    (`self.HandleBuildingClick`)
    (message `/Game/UnitSelection/Unit/BP_RTS_Interface.MarqueePressed` _returnvalue))
  (:`Released`
    (set `self.isLeftMousePressed?` false)
    (message `/Game/UnitSelection/Unit/BP_RTS_Interface.MarqueeReleased` _returnvalue)))

(event `Key|RightMouseButton`
  (params (Key :type "Key Structure"))
  (:`Pressed`
    (set `self.RightClickLocation` (`.Location` (`GameplayStatics.BreakHitResult` (`self.GetHitResultUnderCursorByChannel` "TraceTypeQuery1"))))
    (bind _units (message `/Game/UnitSelection/Unit/BP_RTS_Interface.GrabSelectedUnits` (`self.GetHUD`)))
    (for _array_element _units
      (message `/Game/UnitSelection/Unit/BP_RTS_Interface.UnitMoveCommand` _array_element (`self.RightClickLocation`)))
    (`NiagaraFunctionLibrary.SpawnSystemAtLocation` "/Game/Cursor/FX_Cursor.FX_Cursor" (`self.RightClickLocation`))))

(event `ServerAddUnitToQueue`
  (params (Building :type "/Game/Building/BP_A_Parent_Building_Class Object Reference") (Unit :type "/Game/UnitSelection/Unit/BP_Parent_Unit_Class Class Reference"))
  (`/Game/Building/BP_A_Parent_Building_Class.AddUnitToQueue` Building Unit))

(event `/Game/UnitSelection/Unit/BP_RTS_Interface.ProduceUnit`
  (params (Building :type "/Game/Building/BP_A_Parent_Building_Class Object Reference") (Unit :type "/Game/UnitSelection/Unit/BP_Parent_Unit_Class Class Reference"))
  (`self.ServerAddUnitToQueue` Building Unit))

(fn `GrabSelectedUnits`
  (returns (Units :type "Array of Actor Object Reference"))
  (return))

(fn `UserConstructionScript`)