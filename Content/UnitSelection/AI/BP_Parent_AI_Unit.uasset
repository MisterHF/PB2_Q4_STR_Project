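; Parent Blueprint for an AI unit that roams, attacks sighted BP_Parent_Unit_Class pawns and dies at zero health.
; Roaming chains random reachable moves with pauses; pawn sensing redirects movement to the target, attacking on arrival or resuming roaming on failure.
; A DoOnce-gated attack freezes movement during a montage, then applies sphere-overlap damage to pawns, with debug drawing.
; Tick updates a camera-facing health bar, assuming 100 maximum health.
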(event `self.ReceiveTick`
  (params (DeltaSeconds :type "Float (single-precision)"))
  (bind _healthbar (`self.HealthBar`))
  ;[1 0 0.002808] Event Tick
  ;[1 0.2531 0.1767] Set Health Bar Widget Percent
  (bind _aswg_health_bar (cast `/Game/UnitSelection/Unit/WG_Health_Bar` (`WidgetComponent.GetWidget` (`self.HealthBar`))))
  (`ProgressBar.SetPercent` (`/Game/UnitSelection/Unit/WG_Health_Bar.HealthBar` _aswg_health_bar) (/ (`self.CurrentHealth`) 100.0))
  ;[1 0.4373 0.8804] Set Health Bar Rotation To Face The Camera
  (`SceneComponent.K2_SetWorldRotation` _healthbar (`KismetMathLibrary.FindLookAtRotation` (`SceneComponent.K2_GetComponentLocation` _healthbar) (`SceneComponent.K2_GetComponentLocation` (`PlayerCameraManager.TransformComponent` (`GameplayStatics.GetPlayerCameraManager` 0)))) false false))

(event `self.ReceiveBeginPlay`
  ;[1 0 0.002929] BeginPlay
  ;[0 0.3124 1] Call Roaming Event
  (`self.Roaming`)
  ;[0.4734 0.755 1] Disable Health Bar Shadow
  (`PrimitiveComponent.SetCastShadow` (`self.HealthBar`) false)
  (set `self.CurrentHealth` (`self.MaxHealth`)))

(event `Death`
  ;[1 0.1404 0.1106] Death Event
  (set `self.DeathBool` true)
  (`GameplayStatics.SpawnEmitterAtLocation` null (`KismetMathLibrary.Conv_DoubleToVector` (`SkeletalMeshComponent.GetPosition` (`self.Mesh`))))
  (`self.K2_DestroyActor`))

(event `self.ReceiveAnyDamage`
  (params (Damage :type "Float (single-precision)") (DamageType :type "DamageType Object Reference") (InstigatedBy :type "Controller Object Reference") (DamageCauser :type "Actor Object Reference"))
  ;[0.6439 1 0.8601] Event damage
  (if (not (`self.DeathBool`))
    (bind _output_get (set `self.CurrentHealth` (`KismetMathLibrary.FClamp` (- (`self.CurrentHealth`) Damage) 0.0 (`self.MaxHealth`))))
    (if (== _output_get 0.0)
      (`self.Death`))))

(event `Roaming`
  ;[0.7195 1 0.6408] Roaming
  (set `CharacterMovementComponent.MaxWalkSpeed` 200.0 (`self.CharacterMovement`))
  (`|AIMoveTo` self (`NavigationSystemV1.K2_GetRandomReachablePointInRadius` (`SceneComponent.K2_GetComponentLocation` (`self.Mesh`)) 1000.0 null null) null
    (:`OnSuccess`
      (`KismetSystemLibrary.Delay` (`KismetMathLibrary.RandomFloatInRange` 1.0 4.0))
      (`self.Roaming`))))

(event `Attack`
  ;[1 0.234 0.7498] Attack System
  (`/Engine/EditorBlueprintResources/StandardMacros.DoOnce` false :!label _label
    (:`Completed`
      (`CharacterMovementComponent.DisableMovement` (`self.CharacterMovement`))
      (`|PlayMontage` (`self.Mesh`) (`self.AnimArray`) 2.0
        (:`OnCompleted`
          (`KismetSystemLibrary.Delay` 1.0))
        (:`OnInterrupted`
          (`KismetSystemLibrary.Delay` 2.0)))
      (`CharacterMovementComponent.SetMovementMode` (`self.CharacterMovement`) "MOVE_Walking" 0)
      (`self.DealDamage`)
      (goto _label :!via `Reset`))))

(event `self.PawnSensing.OnSeePawn`
  (params (Pawn :type "Pawn Object Reference"))
  ;[0.5764 0.6282 1] See Pawn
  (bind _asbp_parent_unit_class (cast `/Game/UnitSelection/Unit/BP_Parent_Unit_Class` Pawn))
  (`|AIMoveTo` self (`SceneComponent.K2_GetComponentLocation` (`Actor.RootComponent` _asbp_parent_unit_class)) _asbp_parent_unit_class
    (:`OnSuccess`
      (`self.Attack`))
    (:`OnFail`
      (`KismetSystemLibrary.RetriggerableDelay` 0.2)
      (`self.Roaming`))))

(event `DealDamage`
  ;[1 0.9713 0.3846] Deal Damage
  (bind _outactors (`KismetSystemLibrary.SphereOverlapActors` (`SceneComponent.K2_GetComponentLocation` (`self.DealingDamageSphereArea`)) (`self.AttackRange`) (`|MakeArray` "ObjectTypeQuery3" :!type "EObjectTypeQuery Enum") "/Script/Engine.Actor" (`|MakeArray` self :!type "Actor Object Reference")))
  (`KismetSystemLibrary.DrawDebugSphere` (`SceneComponent.K2_GetComponentLocation` (`self.DealingDamageSphereArea`)) (`self.AttackRange`) 12 (struct :`R` 1.0 :`G` 0.01024 :`A` 1.0) 2.0)
  (for _array_element _outactors
    (`GameplayStatics.ApplyDamage` _array_element (`self.Base Damage`) (`self.GetController`) self "/Script/Engine.DamageType")))

(fn `UserConstructionScript`)