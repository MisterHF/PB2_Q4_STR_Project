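; Base unit Blueprint for a unit selection system, providing selection feedback and move orders.
; SelectThis and DeselectThis show and hide a SelectionDecal to mark whether the unit is selected.
; UnitMoveCommand stops the AI controller's current movement, then issues AIMoveTo toward the given location.
; GrabSelectedUnits and the construction script are empty.
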(event `/Game/UnitSelection/Unit/BP_RTS_Interface.UnitMoveCommand`
  (params (Location :type "Vector Structure"))
  (bind _returnvalue (`AIBlueprintHelperLibrary.GetAIController` self))
  ;[1 0.09372 0.346] Movement Command
  (`Controller.StopMovement` _returnvalue)
  (`AITask_MoveTo.AIMoveTo` _returnvalue Location null))

(event `/Game/UnitSelection/Unit/BP_RTS_Interface.SelectThis`
  (`SceneComponent.SetVisibility` (`self.SelectionDecal`) true false))

(event `/Game/UnitSelection/Unit/BP_RTS_Interface.DeselectThis`
  (`SceneComponent.SetVisibility` (`self.SelectionDecal`) false false))

(fn `GrabSelectedUnits`
  (returns (Units :type "Array of Actor Object Reference"))
  (return))

(fn `UserConstructionScript`)