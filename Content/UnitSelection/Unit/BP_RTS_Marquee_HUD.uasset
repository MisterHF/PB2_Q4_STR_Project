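; HUD Blueprint for RTS marquee selection, drawing a translucent blue rectangle between the mouse press point and the current cursor.
; Pressed, held and released events track the drag, and while active DrawHUD queries parent-class units inside the rectangle every frame.
; Units inside are selected and stored, clearing building selection via the player controller, while units outside are deselected and removed.
; GrabSelectedUnits exposes the selected list.
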(event `/Game/UnitSelection/Unit/BP_RTS_Interface.MarqueePressed`
  (bind (_locationx _locationy) (`PlayerController.GetMousePosition` (`GameplayStatics.GetPlayerController` 0)))
  ;[0 1 0.1625] Marquee Start
  (set `self.isDrawing?` true)
  (bind _output_get (set `self.StartMousePosition` (`KismetMathLibrary.MakeVector2D` _locationx _locationy)))
  (set `self.CurrentMousePosition` _output_get))

(event `/Game/UnitSelection/Unit/BP_RTS_Interface.MarqueeHeld`
  (bind (_locationx _locationy) (`PlayerController.GetMousePosition` (`GameplayStatics.GetPlayerController` 0)))
  ;[0.01999 0.2392 1] Marquee Held
  (set `self.CurrentMousePosition` (`KismetMathLibrary.MakeVector2D` _locationx _locationy)))

(event `/Game/UnitSelection/Unit/BP_RTS_Interface.MarqueeReleased`
  ;[1 0 0.0421] Marquee Released
  (set `self.isDrawing?` false))

(event `SelectUnit`
  (params (ArrayActor :type "Actor Object Reference"))
  ;[0.56 1 0.826] Select Unit under the rectangle
  (message `/Game/UnitSelection/Unit/BP_RTS_Interface.SelectThis` ArrayActor)
  (bind _returnvalue (`KismetArrayLibrary.Array_AddUnique` (`self.SelectedUnit`) ArrayActor))
  (message `/Game/UnitSelection/Unit/BP_RTS_Interface.ClearSelectedBuilding` (`GameplayStatics.GetPlayerController` _returnvalue)))

(event `self.ReceiveDrawHUD`
  (params (SizeX :type Integer) (SizeY :type Integer))
  (bind (_startmouseposition_x _startmouseposition_y) (`KismetMathLibrary.BreakVector2D` (`self.StartMousePosition`)))
  (bind (_currentmouseposition_x _currentmouseposition_y) (`KismetMathLibrary.BreakVector2D` (`self.CurrentMousePosition`)))
  ;[0 0.8867 1] Draw Rectangle
  (if (`self.isDrawing?`)
    (`self.DrawRect` (struct :`G` 0.109804 :`B` 0.921569 :`A` 0.2) _startmouseposition_x _startmouseposition_y (- _currentmouseposition_x _startmouseposition_x) (- _currentmouseposition_y _startmouseposition_y))
    ;[0 0.4199 1] Check for actor under the rectangle
    (bind _output_get (set `self.ActorInRectangle` (`self.GetActorsInSelectionRectangle` "/Game/UnitSelection/Unit/BP_Parent_Unit_Class.BP_Parent_Unit_Class_C" (`self.StartMousePosition`) (`self.CurrentMousePosition`) false)))
    (for _array_element _output_get
      (`self.SelectUnit` _array_element))
    (`self.DeselectUnit`)))

(event `DeselectUnit`
  ;[1 0.3941 0.4373] Deselect Unit under the rectangle
  (for _array_element (`self.SelectedUnit`)
    (if (== (`KismetArrayLibrary.Array_Find` (`self.ActorInRectangle`) _array_element) -1)
      (message `/Game/UnitSelection/Unit/BP_RTS_Interface.DeselectThis` _array_element)
      (`KismetArrayLibrary.Array_RemoveItem` (`self.SelectedUnit`) _array_element))))

(fn `GrabSelectedUnits`
  (returns (Units :type "Array of Actor Object Reference"))
  (return (`self.SelectedUnit`)))

(fn `UserConstructionScript`)