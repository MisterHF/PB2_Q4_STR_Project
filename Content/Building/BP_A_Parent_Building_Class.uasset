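; Parent Blueprint for RTS-style buildings that can be selected and produce units from a queue.
; Selection toggles a decal and a per-building UI widget, created at BeginPlay and filled with the building's action buttons.
; An authority-only looping timer advances production using each unit class's default production time, then spawns the unit at the spawn point.
; It also carries an AI move command, while the progress OnRep and GrabSelectedUnits are empty.
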(event `/Game/UnitSelection/Unit/BP_RTS_Interface.UnitMoveCommand`
  (params (Location :type "Vector Structure"))
  (bind _returnvalue (`AIBlueprintHelperLibrary.GetAIController` self))
  ;[1 0.09372 0.346] Movement Command
  (`Controller.StopMovement` _returnvalue)
  (`AITask_MoveTo.AIMoveTo` _returnvalue Location null))

(event `AddUnitToQueue`
  (params (Unit :type "/Game/UnitSelection/Unit/BP_Parent_Unit_Class Class Reference"))
  ;[0.7675 0.4819 1] Add Unit To Queue
  (`KismetArrayLibrary.Array_Add` (`self.UnitProductionQueue`) Unit))

(event `/Game/UnitSelection/Unit/BP_RTS_Interface.SelectThis`
  (`SceneComponent.SetVisibility` (`self.SelectedDecal`) true false)
  (`UserWidget.AddToViewport` (`self.BuildingSelectedWidget`) 0))

(event `/Game/UnitSelection/Unit/BP_RTS_Interface.DeselectThis`
  (`SceneComponent.SetVisibility` (`self.SelectedDecal`) false false)
  (`Widget.RemoveFromParent` (`self.BuildingSelectedWidget`)))

(event `self.ReceiveBeginPlay`
  (`|ExecutionSequence`
    (:`then_0`
      ;[0.465 0.9834 1] Create building selected widget
      (bind _returnvalue (`|CreateWidget` "/Game/Building/WG_Selected_Building_UI.WG_Selected_Building_UI_C"))
      (set `self.BuildingSelectedWidget` _returnvalue)
      (set `/Game/Building/WG_Selected_Building_UI.BuildingReference` self _returnvalue)
      (for _array_element (`self.ActionBoxButtons`)
        (`WrapBox.AddChildToWrapBox` (`/Game/Building/WG_Selected_Building_UI.ActionBox` (`self.BuildingSelectedWidget`)) _array_element)))
    (:`then_1`
      (`/Engine/EditorBlueprintResources/ActorMacros.Switch Has Authority`
        (:`Authority`
          (`KismetSystemLibrary.K2_SetTimerDelegate` (delegate `ProcessProductionQueue`) (`self.ProductionTimerGranularity`) true))))))

(event `ProcessProductionQueue`
  (if (`self.isProducingUnit?`)
    ;[1 0.5135 0.4703] Create Unit
    (bind _output_get (set `self.ProductionTimeSpend` (+ (`self.ProductionTimeSpend`) (`self.ProductionTimerGranularity`))))
    (bind _output_get_2 (set `self.ProductionProgress` (/ _output_get (`self.ProductionTimeNeeded`))))
    (if (>= _output_get_2 1.0)
      (`|SpawnActorFromClass` (`self.UnitBeingProduced`) (`KismetMathLibrary.MakeTransform` (`SceneComponent.K2_GetComponentLocation` (`self.UnitSpawnPoint`))) "AdjustIfPossibleButAlwaysSpawn" "MultiplyWithRoot" null null)
      (set `self.ProductionProgress` 0.0)
      (set `self.ProductionTimeSpend` 0.0)
      (set `self.UnitBeingProduced` null)
      (set `self.isProducingUnit?` false))
    (elif (> (`KismetArrayLibrary.Array_Length` (`self.UnitProductionQueue`)) 0)
      (bind _output_get_3 (set `self.UnitBeingProduced` (`|GetArrayItem` (`self.UnitProductionQueue`))))
      (set `self.ProductionTimeNeeded` (defaults `Object` _output_get_3))
      (`KismetArrayLibrary.Array_Remove` (`self.UnitProductionQueue`))
      (set `self.isProducingUnit?` true))))

(fn `GrabSelectedUnits`
  (returns (Units :type "Array of Actor Object Reference"))
  (return))

(fn `OnRep_ProductionProgress`)

(fn `UserConstructionScript`)