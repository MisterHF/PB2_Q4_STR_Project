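; Building Blueprint that supplies two unit-production buttons for its action box.
; On BeginPlay it creates the WG_ProductionUnit1 and WG_ProductionUnit2 widgets, adds each uniquely to ActionBoxButtons and sets their BuildingReference to itself.
; The parent BeginPlay runs only after both buttons are registered, and the construction script just calls the parent version.
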(event `self.ReceiveBeginPlay`
  (`|ExecutionSequence`
    (:`then_0`
      (bind _returnvalue (`|CreateWidget` "/Game/Building/WG_Production-Unit1.WG_Production-Unit1_C"))
      (`KismetArrayLibrary.Array_AddUnique` (`self.ActionBoxButtons`) _returnvalue)
      (set `/Game/Building/WG_Production-Unit1.BuildingReference` self _returnvalue))
    (:`then_1`
      (bind _returnvalue_2 (`|CreateWidget` "/Game/Building/WG_Production-Unit2.WG_Production-Unit2_C"))
      (`KismetArrayLibrary.Array_AddUnique` (`self.ActionBoxButtons`) _returnvalue_2)
      (set `/Game/Building/WG_Production-Unit2.BuildingReference` self _returnvalue_2))
    (:`then_2`
      (`parent.ReceiveBeginPlay`))))

(fn `UserConstructionScript`
  (`parent.UserConstructionScript`))